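; BP_BaseEnemy is an enemy base Blueprint that wires up combat feedback widgets.
; On BeginPlay it links the health bar widget to its HealthComponent and hides the attack widget.
; Bound damage events spawn floating damage counters at the damaged actor's location, while a bound feedback event toggles the attack widget's visibility.
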(event `self.ReceiveBeginPlay`
  (bind _aswbp_enemy_health_bar (cast `/Game/UI/Components/WBP_EnemyHealthBar` (`WidgetComponent.GetWidget` (`self.HealthBar`))))
  (`/Game/UI/Components/WBP_EnemyHealthBar.Initialize` _aswbp_enemy_health_bar (`self.HealthComponent`))
  (add `self.OnTakeAnyDamage` (`|CreateDelegate` :!event `SpawnDamageNumber`))
  (`SceneComponent.SetVisibility` (`self.AttackWidget`) false false)
  (add `self.OnSetFeedback` (`|CreateDelegate` :!event `SetFeedback`)))

(event `SpawnDamageNumber` :!signature `self.OnTakeAnyDamage`
  (params (DamagedActor :type "Actor Object Reference") (Damage :type "Float (single-precision)") (DamageType :type "DamageType Object Reference") (InstigatedBy :type "Controller Object Reference") (DamageCauser :type "Actor Object Reference"))
  (`/Game/LibFuncs/BPLib_Utility.SpawnDamageCounter` Damage (`self.K2_GetActorLocation` DamagedActor)))

(event `SetFeedback` :!signature `self.OnSetFeedback`
  (params (isVisible :type Boolean))
  (`SceneComponent.SetVisibility` (`self.AttackWidget`) isVisible false))

(fn `UserConstructionScript`)