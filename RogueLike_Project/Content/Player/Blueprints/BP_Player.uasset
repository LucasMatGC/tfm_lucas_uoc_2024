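; Player character Blueprint that connects player and weapon events to UI, damage feedback and animation.
; When the player is ready, it creates the main HUD and binds each inventory weapon's fire event to alternating sword montages for melee combos.
; Pausing opens the pause menu or continues the game if already paused.
; Damage spawns a counter, then plays a hit montage or flags the animation Blueprint as dead when health runs out.
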(event `self.ReceiveBeginPlay`
  (add `self.OnPlayerReady` (`|CreateDelegate` :!event `OnPlayerReady_Event`))
  (add `self.OnPlayerPause` (`|CreateDelegate` :!event `OnPlayerPause_Event`))
  (add `self.OnTakeAnyDamage` (`|CreateDelegate` :!event `SpawnDamageCounter`)))

(event `BindAttackAnimations`
  (for _array_element (`InventoryComponent.Weapons` (`self.InventoryComponent`))
    (add `BaseWeapon.OnWeaponFire` _array_element (`|CreateDelegate` :!event `TriggerFireAnimation`))))

(event `OnPlayerReady_Event`
  (bind _returnvalue (`|CreateWidget` "/Game/UI/WBP_MainHUD.WBP_MainHUD_C"))
  (bind _output_get (set `self.PlayerHud` _returnvalue))
  (`UserWidget.AddToViewport` _output_get 0)
  (`/Game/UI/WBP_MainHUD.Initialize` (`self.PlayerHud`) self)
  (`self.BindAttackAnimations`))

(event `OnPlayerPause_Event`
  (if (`GameplayStatics.IsGamePaused`)
    (`/Game/UI/WBP_PauseMenu.ContinueGame` (`self.PauseHud`))
    (else
      (bind _returnvalue (`|CreateWidget` "/Game/UI/WBP_PauseMenu.WBP_PauseMenu_C"))
      (bind _output_get (set `self.PauseHud` _returnvalue))
      (`UserWidget.AddToViewport` _output_get 0))))

(event `SpawnDamageCounter` :!signature `self.OnTakeAnyDamage`
  (params (DamagedActor :type "Actor Object Reference") (Damage :type "Float (single-precision)") (DamageType :type "DamageType Object Reference") (InstigatedBy :type "Controller Object Reference") (DamageCauser :type "Actor Object Reference"))
  (`/Game/LibFuncs/BPLib_Utility.SpawnDamageCounter` Damage (`self.K2_GetActorLocation` DamagedActor))
  (if (> (`HealthComponent.CurrentHealth` (`self.HealthComponent`)) 0.0)
    (`self.PlayAnimMontage` "/Game/Player/Animations/Attack/AM_Hit.AM_Hit")
    (else
      (bind _asabp_player_animation (cast `/Game/Player/Animations/ABP_PlayerAnimation` (`SkeletalMeshComponent.GetAnimInstance` (`self.Mesh`))))
      (set `/Game/Player/Animations/ABP_PlayerAnimation.IsPlayerAlive` false _asabp_player_animation))))

(event `TriggerFireAnimation`
  (params (bIsMeleeWeapon :type Boolean) (CurrentCombo :type Integer))
  (if bIsMeleeWeapon
    (if (== (mod CurrentCombo 2) 0)
      (`self.PlayAnimMontage` "/Game/Player/Animations/Attack/AM_SwordAttack02.AM_SwordAttack02")
      (else
        (`self.PlayAnimMontage` "/Game/Player/Animations/Attack/AM_SwordAttack01.AM_SwordAttack01")))))

(fn `UserConstructionScript`)