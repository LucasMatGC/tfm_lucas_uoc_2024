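; Procedural dungeon generator actor that, on BeginPlay, spawns a start room and grows the dungeon by attaching random room types to random open exits.
; Each new room's overlap box is checked: clear rooms add their exits to the pool, while overlapping rooms are destroyed and their exit sealed with a door.
; Generation recurses until the MaxRooms budget or exits run out after a successful placement, then doors close the remaining exits.
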(event `self.ReceiveBeginPlay`
  (`self.SpawnStartRoom`)
  (`self.SpawnNextRoom`))

(event `SpawnStartRoom`
  ;[0.2327 1 0.3823 1 25] Spawn Start Room
  (bind _returnvalue (`|SpawnActorFromClass` "/Game/ProceduralDungeon/BP_DungeonRoom_01.BP_DungeonRoom_01_C" (`SceneComponent.K2_GetComponentToWorld` (`self.DefaultSceneRoot`)) "AlwaysSpawn" "MultiplyWithRoot" null null))
  (`self.AddExits` _returnvalue))

(event `SpawnNextRoom`
  ;[0.2327 1 0.3823 1 25] Spawn Next Room
  (bind _output_get (set `self.SelectedExitPoint` (`KismetArrayLibrary.Array_Random` (`self.ExitsList`))))
  (bind _returnvalue (`|SpawnActorFromClass` (`KismetArrayLibrary.Array_Random` (`self.RoomTypeList`)) (`SceneComponent.K2_GetComponentToWorld` _output_get) "AlwaysSpawn" "MultiplyWithRoot" null null))
  (bind _asbp_master_room (cast `/Game/ProceduralDungeon/BP_Master_Room` _returnvalue))
  (set `self.LatestRoom` _asbp_master_room)
  (`self.CheckOverlapRoom`))

(event `CheckOverlapRoom`
  ;[0.2327 1 0.3823 1 25] Check Overlap
  (bind _asbox_collision (cast `BoxComponent` (`SceneComponent.GetChildComponent` (`/Game/ProceduralDungeon/BP_Master_Room.Overlap Folder` (`self.LatestRoom`)) 0)))
  (if (== (`KismetArrayLibrary.Array_Length` (`PrimitiveComponent.GetOverlappingComponents` _asbox_collision)) 0)
    (`KismetArrayLibrary.Array_Add` (`self.RoomList`) (`self.LatestRoom`))
    (`self.AddExits` (`self.LatestRoom`))
    (`KismetArrayLibrary.Array_RemoveItem` (`self.ExitsList`) (`self.SelectedExitPoint`))
    (bind _returnvalue (`self.CanGenerateAnotherRoom`))
    (if _returnvalue
      (`self.SpawnNextRoom`)
      (else
        (`self.CloseRemainingExits`)))
    (else
      (`self.K2_DestroyActor` (`self.LatestRoom`))
      (`|SpawnActorFromClass` "/Game/ProceduralDungeon/BP_ExitDoor.BP_ExitDoor_C" (`SceneComponent.K2_GetComponentToWorld` (`self.SelectedExitPoint`)) "AlwaysSpawn" "MultiplyWithRoot" null null)
      (`KismetArrayLibrary.Array_RemoveItem` (`self.ExitsList`) (`self.SelectedExitPoint`))
      (`self.SpawnNextRoom`))))

(event `CloseRemainingExits`
  ;[0.2327 1 0.3823] Close Remaining Exits
  (for _array_element (`self.ExitsList`)
    (`|SpawnActorFromClass` "/Game/ProceduralDungeon/BP_ExitDoor.BP_ExitDoor_C" (`SceneComponent.K2_GetComponentToWorld` _array_element) "AlwaysSpawn" "MultiplyWithRoot" null null)))

(fn `AddExits`
  (params (Room :type "/Game/ProceduralDungeon/BP_Master_Room Object Reference"))
  (`KismetArrayLibrary.Array_Append` (`self.ExitsList`) (`SceneComponent.GetChildrenComponents` (`/Game/ProceduralDungeon/BP_Master_Room.Exit Folder` Room) false)))

(fn `CanGenerateAnotherRoom`
  (returns (ReturnValue :type Boolean))
  (bind _result (`/Engine/EditorBlueprintResources/StandardMacros.DecrementInt` (`self.MaxRooms`))
    (:`  `
      (return (and (> _result 0) (> (`KismetArrayLibrary.Array_Length` (`self.ExitsList`)) 0))))))

(fn `UserConstructionScript`)